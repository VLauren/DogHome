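; EndBallBP is a ball with a physically animated skeletal mesh that triggers nightfall when the Dog reaches it while the Squirrel is AWAY.
; It hides itself, notifies Dog and HomeSquare, and briefly disables dog movement.
; A timeline blends the sky sphere, directional light and fog into night.
; If Dog.End is still false three minutes later, it prints game over, plays an outro sequence and reloads the level.
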(event EventBeginPlay
  (bind _skeletalmesh (Variables|Default|GetSkeletalMesh))
  (bind _bonename (Variables|Default|GetBoneName))
  (bind _outactors (Actor|GetAllActorsOfClass "/Script/DogHome.Dog"))
  (Variables|Default|SetDog (Utilities|Array|Get(acopy) _outactors))
  (bind _outactors_2 (Actor|GetAllActorsOfClass "/Script/DogHome.Squirrel"))
  (Variables|Default|SetSquirrel (Utilities|Array|Get(acopy) _outactors_2))
  (bind _outactors_3 (Actor|GetAllActorsOfClass "/Game/Blueprints/Squares/HomeSquareBP.HomeSquareBP_C"))
  (Variables|Default|SetHomeSquare (Utilities|Array|Get(acopy) _outactors_3))
  (bind _outactors_4 (Actor|GetAllActorsOfClass "/Engine/EngineSky/BP_Sky_Sphere.BP_Sky_Sphere_C"))
  (Variables|Default|SetSkySphere (Utilities|Array|Get(acopy) _outactors_4))
  (bind _outactors_5 (Actor|GetAllActorsOfClass "/Script/Engine.DirectionalLight"))
  (Variables|Default|Setdirlight (Utilities|Array|Get(acopy) _outactors_5))
  (bind _outactors_6 (Actor|GetAllActorsOfClass "/Script/Engine.AtmosphericFog"))
  (Variables|Default|Setfog (Utilities|Array|Get(acopy) _outactors_6))
  (Class|PhysicalAnimationComponent|SetSkeletalMeshComponent (Variables|Default|GetPhysicalAnimation) _skeletalmesh)
  (Class|PhysicalAnimationComponent|ApplyPhysicalAnimationProfileBelow (Variables|Default|GetPhysicalAnimation) _bonename "Salchicha" false true)
  (Class|SkeletalMeshComponent|SetAllBodiesBelowSimulatePhysics _skeletalmesh _bonename true false))

(event EventTick
  (params (DeltaSeconds :type Float%20%28single-precision%29))
  (bind _fog (Variables|Default|Getfog))
  (bind _dog (Variables|Default|GetDog))
  (bind _skysphere (Variables|Default|GetSkySphere))
  (bind _dirlight (Variables|Default|Getdirlight))
  (if (Utilities|Enum|Equal(Enum) (Variables|/Script/DogHome.Squirrel|GetState (Variables|Default|GetSquirrel)) "RUN_AWAY")
    (if (and (not (Variables|Default|GetNight)) (< (Math|Vector|VectorLength (- (Transformation|GetActorLocation (Variables|Default|GetDog)) (Transformation|GetWorldLocation (Variables|Default|GetSkeletalMesh)))) 8e+01))
      ;[1 1 1] Se hace de noche
      (Variables|Default|SetNight true)
      (Class|Dog|StartNight (Variables|Default|GetDog))
      (Class|HomeSquare|StartNight (Variables|Default|GetHomeSquare))
      (Class|Dog|DisableMove (Variables|Default|GetDog))
      (Development|SetHiddeninGame (Variables|Default|GetSkeletalMesh) true false)
      (Utilities|FlowControl|Delay 3.0)
      (bind _newtrack_0 (Timeline|Timeline_0 Play)
        (:Update
          (Variables|/Engine/EngineSky/BP_Sky_Sphere.BP_Sky_Sphere_C|SetSun%20height _skysphere (Math|Float|Lerp 0.4 -1.0 _newtrack_0))
          (Default|RefreshMaterial _skysphere)
          (Rendering|Components|Light|SetIntensity (Variables|/Script/Engine.Light|GetLightComponent _dirlight) (Math|Float|Lerp 9.0 3.0 _newtrack_0))
          (Rendering|Components|Light|SetLightColor (Variables|/Script/Engine.Light|GetLightComponent _dirlight) (Utilities|Struct|MakeLinearColor (Math|Float|Lerp 0.896269 0.541667 _newtrack_0) (Math|Float|Lerp 0.473531 0.628019 _newtrack_0) (Math|Float|Lerp 0.473531 1.0 _newtrack_0) 1.0) true)
          (Rendering|SetActorHiddenInGame _fog false)
          (Class|AtmosphericFogComponent|SetStartDistance (Variables|/Script/Engine.AtmosphericFog|GetAtmosphericFogComponent _fog) (Math|Float|Lerp 1e+04 838.0 _newtrack_0))
          (Utilities|FlowControl|Delay 0.2)
          (Class|Dog|EnableMove (Variables|Default|GetDog))
          (Utilities|FlowControl|Delay 1.8e+02)
          (if (not (Variables|/Script/DogHome.Dog|GetEnd _dog))
            (Class|Dog|DisableMove _dog)
            (Development|PrintString "GAME OVER")
            (Utilities|FlowControl|Delay 2.0)
            (bind _outactor (Sequencer|Player|CreateLevelSequencePlayer "/Game/SequenceOut.SequenceOut"))
            (Sequencer|Player|Play (Variables|/Script/LevelSequence.LevelSequenceActor|GetSequencePlayer _outactor) :!class /Script/MovieScene.MovieSceneSequencePlayer)
            (Utilities|FlowControl|Delay 2.0)
            (bind _returnvalue (Game|GetCurrentLevelName true))
            (Game|OpenLevel(byName) (Utilities|String|StringToName _returnvalue))))))))

(fn ConstructionScript)