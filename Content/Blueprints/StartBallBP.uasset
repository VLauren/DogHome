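; StartBallBP is a ball actor that triggers the opening squirrel chase when the Dog gets close.
; On BeginPlay it caches the first Dog and Squirrel found in the level.
; Each Tick, while the Squirrel is in its START state and the Dog is within range of the ball, it disables the Dog's movement and sends the Squirrel to chase the ball's position.
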(event EventBeginPlay
  (bind _outactors (Actor|GetAllActorsOfClass "/Script/DogHome.Dog"))
  (Variables|Default|SetDog (Utilities|Array|Get(acopy) _outactors))
  (bind _outactors_2 (Actor|GetAllActorsOfClass "/Script/DogHome.Squirrel"))
  (Variables|Default|SetSquirrel (Utilities|Array|Get(acopy) _outactors_2)))

(event EventTick
  (params (DeltaSeconds :type Float%20%28single-precision%29))
  (if (Utilities|Enum|Equal(Enum) (Variables|/Script/DogHome.Squirrel|GetState (Variables|Default|GetSquirrel)) "START")
    (if (< (Math|Vector|VectorLength (- (Transformation|GetActorLocation (Variables|Default|GetDog)) (Transformation|GetActorLocation))) 3e+02)
      ;[1 1 1] El perro espera y activo la ardilla
      (Class|Dog|DisableMove (Variables|Default|GetDog))
      (Class|Squirrel|StartChaseBall (Variables|Default|GetSquirrel) (Transformation|GetActorLocation)))))

(fn ConstructionScript)