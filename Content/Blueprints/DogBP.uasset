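; Dog actor Blueprint that handles level-ending moments and a jump smoke effect.
; When the squirrel gets away, it plays the SequenceOut level sequence after a short delay, then reloads the current level.
; Arriving home plays the same sequence, then opens the MenuImagen level.
; The jump particle event spawns a smoke system at the dog's X/Y with a fixed height.
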(event Custom|OnJumpParticle
  (bind _returnvalue (Transformation|GetActorLocation))
  (bind (_x _y) (Math|Vector|BreakVector _returnvalue))
  (Niagara|SpawnSystematLocation "/Game/Particles/HumoSystem.HumoSystem" (Math|Vector|MakeVector _x _y 52.0)))

(event EventOnArriveHome
  (Utilities|FlowControl|Delay 1.0)
  (bind _outactor (Sequencer|Player|CreateLevelSequencePlayer "/Game/SequenceOut.SequenceOut"))
  (Sequencer|Player|Play (Variables|/Script/LevelSequence.LevelSequenceActor|GetSequencePlayer _outactor) :!class /Script/MovieScene.MovieSceneSequencePlayer)
  (Utilities|FlowControl|Delay 3.0)
  (Game|OpenLevel(byName) "MenuImagen"))

(event EventOnSquirrelGotAway
  (Utilities|FlowControl|Delay 1.0)
  (bind _outactor (Sequencer|Player|CreateLevelSequencePlayer "/Game/SequenceOut.SequenceOut"))
  (Sequencer|Player|Play (Variables|/Script/LevelSequence.LevelSequenceActor|GetSequencePlayer _outactor) :!class /Script/MovieScene.MovieSceneSequencePlayer)
  (Utilities|FlowControl|Delay 4.0)
  (bind _returnvalue (Game|GetCurrentLevelName true))
  (Game|OpenLevel(byName) (Utilities|String|StringToName _returnvalue)))

(fn ConstructionScript)