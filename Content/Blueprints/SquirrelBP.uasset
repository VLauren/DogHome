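; Squirrel actor that drives stages of a chase with the Dog through a State enum checked on Tick.
; In BALL state, nearing the StartBall switches to PATH, hides the ball, reveals the squirrel, updates the Dog's target lock and movement, and raises the race music parameter.
; In DOG state it hides and spawns an EndBall once, switching to AWAY when the Dog approaches.
; BeginPlay caches these actors and sets partial-body physical animation.
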(event EventBeginPlay
  (bind _bonename (Variables|Default|GetBoneName))
  (bind _skeletalmesh (Variables|Default|GetSkeletalMesh))
  (bind _outactors (Actor|GetAllActorsOfClass "/Script/DogHome.Dog"))
  (bind _outactors_2 (Actor|GetAllActorsOfClass "/Game/Blueprints/Squares/HomeSquareBP.HomeSquareBP_C"))
  (Variables|Default|SetHomeSquare (Utilities|Array|Get(acopy) _outactors_2))
  (Variables|Default|SetDog (Utilities|Array|Get(acopy) _outactors))
  (bind _outactors_3 (Actor|GetAllActorsOfClass "/Game/Blueprints/StartBallBP.StartBallBP_C"))
  (Variables|Default|SetBall (Utilities|Array|Get(acopy) _outactors_3))
  (Class|PhysicalAnimationComponent|SetSkeletalMeshComponent (Variables|Default|GetPhysicalAnimation) _skeletalmesh)
  (Class|PhysicalAnimationComponent|ApplyPhysicalAnimationProfileBelow (Variables|Default|GetPhysicalAnimation) _bonename "Salchicha" false true)
  (Class|SkeletalMeshComponent|SetAllBodiesBelowSimulatePhysics _skeletalmesh _bonename true false))

(event EventTick
  (params (DeltaSeconds :type Float%20%28single-precision%29))
  (bind _returnvalue (Transformation|GetActorTransform))
  (bind _ball (Variables|Default|GetBall))
  (Utilities|FlowControl|Sequence
    (:then_0
      (if (Utilities|Enum|Equal(Enum) (Variables|Default|GetState) "WAIT_DOG")
        (Development|SetHiddeninGame (Variables|Default|GetSkeletalMesh) true false)
        (Utilities|FlowControl|DoOnce false
          (:Completed
            (bind _returnvalue_2 (Game|SpawnActorfromClass "/Game/Blueprints/EndBallBP.EndBallBP_C" (Math|Transform|MakeTransform (Math|Vector|MakeVector (.x (.location _returnvalue)) (.y (.location _returnvalue)) 0.0) "0, 0, 0" "1,1,1") "AlwaysSpawn" 0 0))
            (Variables|Default|SetEndBall _returnvalue_2)))
        (else
          (if (Utilities|IsValid _ball) :!label _label
            (if (and (Utilities|Enum|Equal(Enum) (Variables|Default|GetState) "CHASE_BALL") (< (Math|Vector|VectorLength (- (Transformation|GetWorldLocation (Variables|/Game/Blueprints/StartBallBP.StartBallBP_C|Getsalchicha _ball)) (Transformation|GetActorLocation))) 8e+01))
              (Variables|Default|SetState "FOLLOW_PATH")
              (Class|Dog|SetLockTarget (Variables|Default|GetDog))
              (Rendering|SetActorHiddenInGame (Variables|Default|GetBall) true)
              (Class|Dog|EnableMove (Variables|Default|GetDog))
              (Development|SetHiddeninGame (Variables|Default|GetSkeletalMesh) false false)
              (Class|FMODBlueprintStatics|EventInstanceSetParameter (Variables|/Game/Blueprints/Squares/HomeSquareBP.HomeSquareBP_C|GetMusica (Variables|Default|GetHomeSquare)) "carrera" 1.0))))))
    (:then_1
      (goto _label))
    (:then_2
      (if (and (Utilities|Enum|Equal(Enum) (Variables|Default|GetState) "WAIT_DOG") (< (Math|Vector|VectorLength (- (Transformation|GetActorLocation (Variables|Default|GetDog)) (Transformation|GetActorLocation))) 3e+02))
        (Variables|Default|SetState "RUN_AWAY")
        (Class|Dog|SetLockTarget (Variables|Default|GetDog))))))

(fn ConstructionScript)