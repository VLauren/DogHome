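; Home square Blueprint that switches scenery lighting and FMOD audio between the starting state and night.
; BeginPlay applies unlit materials to meshes, starts forest-chase ambience and music, then sets start parameters after delays, with mismatched spellings "presstart" and "pressstart".
; OnNight swaps those material slots to lit versions and sets the music's race-end and proximity parameters.
; Disconnected chains hold older house and streetlamp material logic, including the material variable assignments.
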(event EventOnNight
  (Rendering|Material|SetMaterial (Variables|Default|GetStaticMesh1) 4 (Variables|Default|GetLuz))
  (Rendering|Material|SetMaterial (Variables|Default|GetBanco1) 1 (Variables|Default|GetLuz))
  (Class|FMODBlueprintStatics|EventInstanceSetParameter (Variables|Default|GetMusica) "fincarrera" 1.0)
  (Class|FMODBlueprintStatics|EventInstanceSetParameter (Variables|Default|GetMusica) "cercanía" 0.5))

(event EventBeginPlay
  (Rendering|Material|SetMaterial (Variables|Default|GetBanco1) 1 (Variables|Default|GetNoLuz))
  (Rendering|Material|SetMaterial (Variables|Default|GetStaticMesh1) 4 (Variables|Default|GetNoLuz))
  (bind _returnvalue (Class|FMODBlueprintStatics|PlayEvent2D "/Game/FMOD/Events/AMBIENTES/Bosque_Persecucion_Ardilla.Bosque_Persecucion_Ardilla"))
  (Variables|Default|SetAmbiente _returnvalue)
  (bind _returnvalue_2 (Class|FMODBlueprintStatics|PlayEvent2D "/Game/FMOD/Events/Musica.Musica"))
  (bind _output_get (Variables|Default|SetMusica _returnvalue_2))
  (Utilities|FlowControl|Delay 0.2)
  (Class|FMODBlueprintStatics|EventInstanceSetParameter _output_get "presstart" 1.0)
  (Utilities|FlowControl|Delay 1.0)
  (Class|FMODBlueprintStatics|EventInstanceSetParameter (Variables|Default|GetMusica) "pressstart" 0.0))

(fn ConstructionScript)