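; SpawnCesped is a component that scatters grass (césped) around its owning actor when play begins.
; Two sequential passes each spawn a random count of actors, one for Cesped and one for Cesped1, with collision ignored.
; Each spawn gets a random horizontal offset from the owner's location within the Negativo–Positivo range, and a random yaw derived from a random flat direction vector.
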(event EventBeginPlay
  (bind _negativo (Variables|Default|GetNegativo))
  (bind _positivo (Variables|Default|GetPositivo))
  (bind _negativo_2 (Variables|Default|GetNegativo))
  (bind _positivo_2 (Variables|Default|GetPositivo))
  (bind _returnvalue (Math|Random|RandomFloatinRange _negativo _positivo))
  (bind _returnvalue_2 (Math|Random|RandomFloatinRange _negativo _positivo))
  (bind _returnvalue_3 (Math|Random|RandomFloatinRange _negativo_2 _positivo_2))
  (bind _returnvalue_4 (Math|Random|RandomFloatinRange _negativo_2 _positivo_2))
  (bind _returnvalue_5 (Math|Vector|MakeVector _returnvalue_3 _returnvalue_4 0.0))
  (bind _returnvalue_6 (Math|Vector|MakeVector _returnvalue _returnvalue_2 0.0))
  (Utilities|FlowControl|Sequence
    (:then_0
      (for _index (range 0 (Math|Random|RandomIntegerinRange 1 25))
        (Game|SpawnActorfromClass "/Game/Blueprints/Cesped.Cesped_C" (Math|Transform|MakeTransform (+ _returnvalue_5 (Transformation|GetActorLocation (Components|GetOwner))) (Math|Conversions|RotationFromXVector _returnvalue_5) "1,1,1") "AlwaysSpawn" 0 0)))
    (:then_1
      (for _index_2 (range 0 (Math|Random|RandomIntegerinRange 1 25))
        (Game|SpawnActorfromClass "/Game/Blueprints/Cesped1.Cesped1_C" (Math|Transform|MakeTransform (+ _returnvalue_6 (Transformation|GetActorLocation (Components|GetOwner))) (Math|Conversions|RotationFromXVector _returnvalue_6) "1,1,1") "AlwaysSpawn" 0 0)))))

(event EventTick
  (params (DeltaSeconds :type Float%20%28single-precision%29)))