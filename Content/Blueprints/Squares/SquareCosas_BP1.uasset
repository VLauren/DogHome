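; Square actor that scatters randomized ground decoration, apparently grass, across its area when play begins.
; SpawnGrass fills two InstancedStaticMesh components with random counts of unit-scale instances at random flat positions within a fixed local square.
; The second mesh's loop is nested inside the first's, multiplying its count, though its positions are independent.
; Random yaw comes from RotationFromXVector on a random horizontal vector.
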(event EventBeginPlay
  (CallFunction|SpawnGrass))

(event Collision|EventActorBeginOverlap
  (params (OtherActor :type Actor%20Object%20Reference)))

(event EventTick
  (params (DeltaSeconds :type Float%20%28single-precision%29)))

(fn ConstructionScript)

(fn SpawnGrass
  (bind _returnvalue (Math|Random|RandomFloatinRange -1.2e+03 1.2e+03))
  (bind _returnvalue_2 (Math|Random|RandomFloatinRange -1.2e+03 1.2e+03))
  (bind _returnvalue_3 (Math|Random|RandomFloatinRange -1.2e+03 1.2e+03))
  (bind _returnvalue_4 (Math|Random|RandomFloatinRange -1.2e+03 1.2e+03))
  (bind _returnvalue_5 (Math|Vector|MakeVector _returnvalue _returnvalue_2 0.0))
  (bind _returnvalue_6 (Math|Vector|MakeVector _returnvalue_4 _returnvalue_3 0.0))
  (Utilities|FlowControl|Sequence
    (:then_0
      (for _index (range 0 (Math|Random|RandomIntegerinRange 1 15))
        (Components|InstancedStaticMesh|AddInstance (Variables|Default|GetInstancedStaticMesh) (Math|Transform|MakeTransform _returnvalue_5 (Math|Conversions|RotationFromXVector _returnvalue_5) "1,1,1"))
        (for _index_2 (range 0 (Math|Random|RandomIntegerinRange 5 10))
          (Components|InstancedStaticMesh|AddInstance (Variables|Default|GetInstancedStaticMesh1) (Math|Transform|MakeTransform _returnvalue_6 (Math|Conversions|RotationFromXVector _returnvalue_6) "1,1,1")))))))